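; VR handgun Blueprint that handles gripping, trigger animation and hand placement on the slide; firing and slide movement are not implemented here.
; Main grab swaps per-hand Enhanced Input mapping contexts and caches the holding hand's anim instance.
; Analog trigger input drives finger animation and trigger rotation, with an empty fire-threshold branch.
; Slide grab snaps the grabbing hand mesh to left/right anchors, reattaching it to its controller with hardcoded offsets on release.
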(event EventBeginPlay)

(event Collision|EventActorBeginOverlap
  (params (OtherActor :type Actor%20Object%20Reference)))

(event EventTick
  (params (DeltaSeconds :type Float%20%28single-precision%29)))

(event OnGrabbed(MainGrabComponent)
  (params (Motion%20Controller :type Motion%20Controller%20Component%20Object%20Reference))
  ;[1 1 1] Main Grab
  (Variables|Default|GetMotion%20Controller
    (:then
      (|RemoveMappingContextFromOppositeHandAndClearTheRefernce))
    (:else
      _))
  (Variables|Default|SetMotion%20Controller Motion%20Controller)
  (bind _holdinghandanim (CallFunction|GetHoldingHandAnim))
  (Variables|Default|SetHolding%20Hand%20Anim _holdinghandanim)
  (Input|EnableInput (Game|GetPlayerController 0))
  (Input|AddMappingContext (PlayerController|LocalPlayerSubsystems|GetEnhancedInputLocalPlayerSubsystem (Game|GetPlayerController 0)) (select (Utilities|Enum|Equal(Enum) (Default|GetHeldbyHand (Variables|Default|GetMainGrabComponent)) "Left") "/Game/VRTemplate/Input/IMC_Weapon_Left.IMC_Weapon_Left" "/Game/VRTemplate/Input/IMC_Weapon_Right.IMC_Weapon_Right") 1 "(bIgnoreAllPressedKeysUntilRelease=True,bForceImmediately=False,bNotifyUserSettings=False)"))

(event OnDropped(MainGrabComponent)
  ;[1 1 1] Main Grab
  (Input|DisableInput (Game|GetPlayerController 0))
  (Input|RemoveMappingContext (PlayerController|LocalPlayerSubsystems|GetEnhancedInputLocalPlayerSubsystem (Game|GetPlayerController 0)) (select (Utilities|Enum|Equal(Enum) (Default|GetHeldbyHand (Variables|Default|GetMainGrabComponent)) "Left") "/Game/VRTemplate/Input/IMC_Weapon_Left.IMC_Weapon_Left" "/Game/VRTemplate/Input/IMC_Weapon_Right.IMC_Weapon_Right") "(bIgnoreAllPressedKeysUntilRelease=True,bForceImmediately=False,bNotifyUserSettings=False)"))

(event Input|EnhancedActionEvents|EnhancedInputActionIA_GunShoot_Left
  (params (ActionValue :type Float%20%28double-precision%29) (ElapsedSeconds :type Float%20%28double-precision%29) (TriggeredSeconds :type Float%20%28double-precision%29) (InputAction :type Input%20Action%20Object%20Reference :default "/Game/VRTemplate/Input/Actions/IA_GunShoot_Left.IA_GunShoot_Left"))
  (:Triggered
    (bind _output_get (Variables|Default|SetAction%20Value%20Left ActionValue))
    (Variables|/Game/ProjectFiles/AssetHands/Animations/ABP_HandAnim.ABP_HandAnim_C|SetTriggerPressValue (Variables|Default|GetHolding%20Hand%20Anim) _output_get)
    (Transformation|SetRelativeRotation (Variables|Default|GetTrigger) (Math|Rotator|Lerp(Rotator) "0, 0, 0" (Variables|Default|GetTriggerFinalPossibleRotation) (Variables|Default|GetAction%20Value%20Left)) false false)
    (if (> (Variables|Default|GetAction%20Value%20Left) (Variables|Default|GetFireThreshold))
      _))
  (:Canceled
    (Variables|Default|SetAction%20Value%20Left 0.0 :!label _label)
    (Variables|/Game/ProjectFiles/AssetHands/Animations/ABP_HandAnim.ABP_HandAnim_C|SetTriggerPressValue (Variables|Default|GetHolding%20Hand%20Anim) 0.0))
  (:Completed
    (goto _label)))

(event Input|EnhancedActionEvents|EnhancedInputActionIA_GunShoot_Right
  (params (ActionValue :type Float%20%28double-precision%29) (ElapsedSeconds :type Float%20%28double-precision%29) (TriggeredSeconds :type Float%20%28double-precision%29) (InputAction :type Input%20Action%20Object%20Reference :default "/Game/VRTemplate/Input/Actions/IA_GunShoot_Right.IA_GunShoot_Right"))
  (:Triggered
    (bind _output_get (Variables|Default|SetAction%20Value%20Right ActionValue))
    (Variables|/Game/ProjectFiles/AssetHands/Animations/ABP_HandAnim.ABP_HandAnim_C|SetTriggerPressValue (Variables|Default|GetHolding%20Hand%20Anim) _output_get)
    (Transformation|SetRelativeRotation (Variables|Default|GetTrigger) (Math|Rotator|Lerp(Rotator) "0, 0, 0" (Variables|Default|GetTriggerFinalPossibleRotation) (Variables|Default|GetAction%20Value%20Right)) false false)
    (if (> (Variables|Default|GetAction%20Value%20Right) (Variables|Default|GetFireThreshold))
      _))
  (:Canceled
    (Variables|Default|SetAction%20Value%20Right 0.0 :!label _label)
    (Variables|/Game/ProjectFiles/AssetHands/Animations/ABP_HandAnim.ABP_HandAnim_C|SetTriggerPressValue (Variables|Default|GetHolding%20Hand%20Anim) 0.0))
  (:Completed
    (goto _label)))

(event OnGrabbed(CurlGrabComponent)
  (params (Motion%20Controller :type Motion%20Controller%20Component%20Object%20Reference))
  (CallFunction|AttachHandtoSlide Motion%20Controller))

(event OnDropped(CurlGrabComponent)
  (CallFunction|DetachHandfromSlide))

(fn ConstructionScript)

(fn GetHoldingHandAnim
  (bind _maingrabcomponent (Variables|Default|GetMainGrabComponent))
  (if (Utilities|Enum|Equal(Enum) (Default|GetHeldbyHand _maingrabcomponent) "Left")
    (return (Variables|/Game/VRTemplate/Blueprints/GrabComponent.GrabComponent_C|GetLeftHandAnim _maingrabcomponent))
    (else
      (return (Variables|/Game/VRTemplate/Blueprints/GrabComponent.GrabComponent_C|GetRightHandAnim _maingrabcomponent)))))

(fn AttachHandtoSlide
  (params (MotionController :type Motion%20Controller%20Component%20Object%20Reference))
  (bind _output_get (Variables|Default|SetSlideGrabMotionController MotionController))
  (bind _array_element (Utilities|Array|ForEachLoopwithBreak (Components|GetChildrenComponents _output_get false) :!label _label)
    (:LoopBody
      (bind _asb_mannequins_xr (Utilities|Casting|CastToB_MannequinsXR _array_element))
      (bind _output_get_2 (Variables|Default|SetSlideMotionControllerHandMesh _asb_mannequins_xr))
      (goto _label Break))
    (:Completed
      (if (Utilities|Enum|Equal(Enum) (Default|GetHeldbyHand (Variables|Default|GetCurlGrabComponent)) "Right")
        (Transformation|AttachComponentToComponent _output_get_2 (Variables|Default|GetSlideHand_R) "None" "SnapToTarget" "SnapToTarget" "KeepRelative" true)
        (else
          (Transformation|AttachComponentToComponent _output_get_2 (Variables|Default|GetSlideHand_L) "None" "SnapToTarget" "SnapToTarget" "KeepRelative" true)))
      (return))))

(fn DetachHandfromSlide
  (bind _slidemotioncontrollerhandmesh (Variables|Default|GetSlideMotionControllerHandMesh))
  (Transformation|AttachComponentToComponent (Variables|Default|GetSlideMotionControllerHandMesh) (Variables|Default|GetSlideGrabMotionController) "None" "SnapToTarget" "SnapToTarget" "SnapToTarget" true)
  (if (Utilities|Enum|Equal(Enum) (Default|GetHeldbyHand (Variables|Default|GetCurlGrabComponent)) "Right")
    (Transformation|AddRelativeRotation _slidemotioncontrollerhandmesh "-53.000000,-13.500000,106.800000" false false)
    (else
      (Transformation|AddRelativeRotation _slidemotioncontrollerhandmesh "-53.000000,-13.500000,256.900000" false false)
      (Transformation|SetRelativeScale3D _slidemotioncontrollerhandmesh (* (Variables|/Script/Engine.SceneComponent|GetRelativeScale3D _slidemotioncontrollerhandmesh) "1.000000,-1.000000,1.000000"))))
  (Transformation|SetRelativeLocation _slidemotioncontrollerhandmesh "-6.200000,0.100000,5.600000" false false)
  (return))